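; Game state Blueprint that checks for game over and stage progression every Tick.
; When Life reaches zero or below, it sets the game-over flag, copies Score to the game instance as the final score, then opens the Gameover level after a short delay.
; Otherwise, it increments GameStage on every tick while KillCount meets its threshold, with no counter reset in this graph.
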(event EventBeginPlay)

(event EventTick
  (params (DeltaSeconds :type Float%20%28single-precision%29))
  (if (<= (Variables|Default|GetLife) 0)
    (Variables|Default|SetGameover true)
    (bind _asbp_gameinstance (Utilities|Casting|CastToBP_Gameinstance (Game|GetGameInstance)))
    (Variables|/Game/BluePrint/BP_Gameinstance.BP_Gameinstance_C|SetFinalplayerScore _asbp_gameinstance (Variables|Default|GetScore))
    (Utilities|FlowControl|Delay 0.2)
    (Game|OpenLevel(byObjectReference) "/Game/Gameover/Gameover.Gameover")
    (elif (>= (Variables|Default|GetKillCount) 15)
      (Variables|Default|SetGameStage (+ (Variables|Default|GetGameStage) 1)))))

(fn ConstructionScript)