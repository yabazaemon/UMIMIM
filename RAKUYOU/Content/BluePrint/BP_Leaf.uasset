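; Clickable leaf enemy that sways on a sine offset along local X, mirroring its flipbook to match travel direction.
; External events toggle breakability, the "almost" zone and defeat; clicks drain HP only while breakable.
; Tick destroys killed or defeated leaves, and EndPlay updates BP_GameState: kills add score (doubled in the almost zone), defeats cost a life and refresh the UI.
; The live leaf count rises on BeginPlay and falls on destruction, except on defeat.
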(event OnClicked(ClickedCollision)
  (params (TouchedComponent :type Primitive%20Component%20Object%20Reference) (ButtonPressed :type Key%20Structure :default "None"))
  (if (Variables|Default|GetCanBreak)
    (Variables|Default|SetLeafHP (- (Variables|Default|GetLeafHP) 1))
    (if (<= (Variables|Default|GetLeafHP) 0)
      (Variables|Default|SetLeaveKilled true))))

(event EventBeginPlay
  (Variables|Default|SetLeaveKilled false)
  (Variables|Default|SetLeaveDefeated false)
  (bind _asbp_game_state (Utilities|Casting|CastToBP_GameState (Game|GetGameState)))
  (Variables|/Game/BluePrint/BP_GameState.BP_GameState_C|SetLeavesNowCount _asbp_game_state (+ (Variables|/Game/BluePrint/BP_GameState.BP_GameState_C|GetLeavesNowCount _asbp_game_state) 1)))

(event Collision|EventActorBeginOverlap
  (params (OtherActor :type Actor%20Object%20Reference)))

(event EventTick
  (params (DeltaSeconds :type Float%20%28single-precision%29))
  (CallFunction|LeafFlipTurn DeltaSeconds)
  (if (Variables|Default|GetLeaveKilled)
    (Actor|DestroyActor)
    (elif (Variables|Default|GetLeaveDefeated)
      (Actor|DestroyActor)
      (else
        (bind _output_get (Variables|Default|SetElapsedTime (+ (Variables|Default|GetElapsedTime) DeltaSeconds)))
        (Transformation|AddActorLocalOffset (Math|Vector|MakeVector (* (Math|Trig|Sin(Radians) (* _output_get (Variables|Default|GetFrequency))) (Variables|Default|GetAmplitude)) 0.0 0.0) false false)))))

(event EventEndPlay
  (params (EndPlayReason :type EEndPlayReason%20Enum :default "Destroyed"))
  (switch Utilities|FlowControl|Switch|SwitchonEEndPlayReason EndPlayReason
    (:Destroyed
      (if (Variables|Default|GetLeaveKilled)
        (bind _asbp_game_state (Utilities|Casting|CastToBP_GameState (Game|GetGameState)))
        (if (Variables|Default|GetOn%20almostzone)
          (Variables|/Game/BluePrint/BP_GameState.BP_GameState_C|SetScore _asbp_game_state (+ (Variables|/Game/BluePrint/BP_GameState.BP_GameState_C|GetScore _asbp_game_state) (* (Variables|Default|GetNomal%20Leaf%20Score) 2)))
          (Variables|Default|SetLeaveKilled false)
          (bind _asbp_game_state_2 (Utilities|Casting|CastToBP_GameState (Game|GetGameState)))
          (bind _output_get (Variables|/Game/BluePrint/BP_GameState.BP_GameState_C|SetLeavesNowCount _asbp_game_state_2 (- (Variables|/Game/BluePrint/BP_GameState.BP_GameState_C|GetLeavesNowCount _asbp_game_state_2) 1)))
          (Development|PrintString (Utilities|String|ToString(Integer) _output_get))
          (bind _output_get_2 (Variables|/Game/BluePrint/BP_GameState.BP_GameState_C|SetKillCount _asbp_game_state_2 (+ (Variables|/Game/BluePrint/BP_GameState.BP_GameState_C|GetKillCount _asbp_game_state_2) 1)))
          (Development|PrintString (Utilities|String|ToString(Integer) _output_get_2))
          (else
            (Variables|/Game/BluePrint/BP_GameState.BP_GameState_C|SetScore _asbp_game_state (+ (Variables|/Game/BluePrint/BP_GameState.BP_GameState_C|GetScore _asbp_game_state) (Variables|Default|GetNomal%20Leaf%20Score)))
            (Variables|Default|SetLeaveKilled false)
            (bind _asbp_game_state_3 (Utilities|Casting|CastToBP_GameState (Game|GetGameState)))
            (bind _output_get_3 (Variables|/Game/BluePrint/BP_GameState.BP_GameState_C|SetLeavesNowCount _asbp_game_state_3 (- (Variables|/Game/BluePrint/BP_GameState.BP_GameState_C|GetLeavesNowCount _asbp_game_state_3) 1)))
            (Development|PrintString (Utilities|String|ToString(Integer) _output_get_3))
            (bind _output_get_4 (Variables|/Game/BluePrint/BP_GameState.BP_GameState_C|SetKillCount _asbp_game_state_3 (+ (Variables|/Game/BluePrint/BP_GameState.BP_GameState_C|GetKillCount _asbp_game_state_3) 1)))
            (Development|PrintString (Utilities|String|ToString(Integer) _output_get_4))))
        (elif (Variables|Default|GetLeaveDefeated)
          (bind _asbp_game_state_4 (Utilities|Casting|CastToBP_GameState (Game|GetGameState)))
          (bind _output_get_5 (Variables|/Game/BluePrint/BP_GameState.BP_GameState_C|SetLife _asbp_game_state_4 (- (Variables|/Game/BluePrint/BP_GameState.BP_GameState_C|GetLife _asbp_game_state_4) 1)))
          (Default|ApplyLife (Variables|/Game/BluePrint/BP_GameState.BP_GameState_C|GetMainUI _asbp_game_state_4) _output_get_5)
          (else
            (bind _asbp_game_state_5 (Utilities|Casting|CastToBP_GameState (Game|GetGameState)))
            (bind _output_get_6 (Variables|/Game/BluePrint/BP_GameState.BP_GameState_C|SetLeavesNowCount _asbp_game_state_5 (- (Variables|/Game/BluePrint/BP_GameState.BP_GameState_C|GetLeavesNowCount _asbp_game_state_5) 1)))
            (Development|PrintString (Utilities|String|ToString(Integer) _output_get_6))))))))

(event EventSetDeath
  (Variables|Default|SetLeaveDefeated true))

(event EventSetCanBreak
  (Variables|Default|SetCanBreak true))

(event EventOffSetCanBreak
  (Variables|Default|SetCanBreak false))

(event EventOffSetAlmost
  (Variables|Default|SetOn%20almostzone false))

(event EventSetAlmost
  (Variables|Default|SetOn%20almostzone true))

(fn ConstructionScript)

(fn LeafFlipTurn
  (params (Delta%20Seconds :type Float%20%28double-precision%29))
  (bind _output_get (Variables|Default|SetCurrentLocation (Transformation|GetActorLocation)))
  (Math|Float|CompareFloat (.X (Math|Vector|BreakVector (- _output_get (Variables|Default|GetPreviousLocation)))) 0.0
    (:>
      (Transformation|SetRelativeScale3D (Variables|Default|GetFlipbook) "-1.000000,1.000000,1.000000")
      (Variables|Default|SetPreviousLocation (Variables|Default|GetCurrentLocation)))
    (:<
      (Transformation|SetRelativeScale3D (Variables|Default|GetFlipbook) "1.000000,1.000000,1.000000")
      (Variables|Default|SetPreviousLocation (Variables|Default|GetCurrentLocation)))))