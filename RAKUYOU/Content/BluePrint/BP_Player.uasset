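; BP_Player is a side-scrolling Paper2D player character with move, jump and slash actions driven by Enhanced Input.
; Movement runs along world X, and FlipTurn yaws the controller to face the input direction.
; Every tick UpdateAnimation picks the flipbook, prioritizing slash, then airborne, walk and idle.
; BreakTriggerSphere overlaps toggle CanBreal on BP_Leaf actors, while the slash input itself only sets the IsSlashing flag.
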(event OnComponentBeginOverlap(BreakTriggerSphere)
  (params (OverlappedComponent :type Primitive%20Component%20Object%20Reference) (OtherActor :type Actor%20Object%20Reference) (OtherComp :type Primitive%20Component%20Object%20Reference) (OtherBodyIndex :type Integer) (bFromSweep :type Boolean) (SweepResult :type Hit%20Result%20Structure%20%28by%20ref%29))
  (bind _asbp_leaf (Utilities|Casting|CastToBP_Leaf OtherActor))
  (Variables|/Game/BluePrint/BP_Leaf.BP_Leaf_C|SetCanBreal _asbp_leaf true))

(event OnComponentEndOverlap(BreakTriggerSphere)
  (params (OverlappedComponent :type Primitive%20Component%20Object%20Reference) (OtherActor :type Actor%20Object%20Reference) (OtherComp :type Primitive%20Component%20Object%20Reference) (OtherBodyIndex :type Integer))
  (bind _asbp_leaf (Utilities|Casting|CastToBP_Leaf OtherActor))
  (Variables|/Game/BluePrint/BP_Leaf.BP_Leaf_C|SetCanBreal _asbp_leaf false))

(event Input|EnhancedActionEvents|EnhancedInputActionIA_Move
  (params (ActionValue :type Float%20%28double-precision%29) (ElapsedSeconds :type Float%20%28double-precision%29) (TriggeredSeconds :type Float%20%28double-precision%29) (InputAction :type Input%20Action%20Object%20Reference :default "/Game/Mapping/IA_Move.IA_Move"))
  (Pawn|Input|AddMovementInput "1.000000,0.000000,0.000000" ActionValue false)
  (CallFunction|FlipTurn ActionValue))

(event Input|EnhancedActionEvents|EnhancedInputActionIA_Jump
  (params (ActionValue :type Boolean) (ElapsedSeconds :type Float%20%28double-precision%29) (TriggeredSeconds :type Float%20%28double-precision%29) (InputAction :type Input%20Action%20Object%20Reference :default "/Game/Mapping/IA_Jump.IA_Jump"))
  (:Triggered
    (Character|Jump))
  (:Completed
    (Character|StopJumping)))

(event Input|EnhancedActionEvents|EnhancedInputActionIA_Slash
  (params (ActionValue :type Boolean) (ElapsedSeconds :type Float%20%28double-precision%29) (TriggeredSeconds :type Float%20%28double-precision%29) (InputAction :type Input%20Action%20Object%20Reference :default "/Game/Mapping/IA_Slash.IA_Slash"))
  (:Triggered
    (Variables|Default|SetIsSlashing true))
  (:Completed
    (Variables|Default|SetIsSlashing false)))

(event EventBeginPlay
  (bind _asbp_player_controller (Utilities|Casting|CastToBP_PlayerController (Pawn|GetController)))
  (Utilities|IsValid (PlayerController|LocalPlayerSubsystems|GetEnhancedInputLocalPlayerSubsystem _asbp_player_controller)
    (:Is%20Valid
      (Input|AddMappingContext (PlayerController|LocalPlayerSubsystems|GetEnhancedInputLocalPlayerSubsystem _asbp_player_controller) "/Game/Mapping/IMC_Default.IMC_Default" 0 "(bIgnoreAllPressedKeysUntilRelease=True,bForceImmediately=False,bNotifyUserSettings=False)"))))

(event Collision|EventActorBeginOverlap
  (params (OtherActor :type Actor%20Object%20Reference)))

(event EventTick
  (params (DeltaSeconds :type Float%20%28single-precision%29))
  (CallFunction|UpdateAnimation))

(fn ConstructionScript)

(fn FlipTurn
  (params (Input :type Float%20%28double-precision%29))
  (bind _returnvalue (Pawn|GetController))
  (Math|Float|CompareFloat Input 0.0
    (:>
      (Pawn|SetControlRotation _returnvalue (Math|Rotator|MakeRotator 0.0 0.0 0.0)))
    (:<
      (Pawn|SetControlRotation _returnvalue (Math|Rotator|MakeRotator 0.0 0.0 1.8e+02)))))

(fn UpdateAnimation
  (if (Variables|Default|GetIsSlashing)
    (Sprite|SetFlipbook (Variables|Default|GetSprite) "/Game/Texture/Slash/dotpict_Slash.dotpict_Slash")
    (elif (AI|Components|NavMovement|IsFalling (Variables|Character|GetCharacterMovement))
      (Sprite|SetFlipbook (Variables|Default|GetSprite) "/Game/Texture/Jump/dotpict_Jump.dotpict_Jump")
      (elif (!= (.x (Transformation|GetVelocity)) 0.0)
        (Sprite|SetFlipbook (Variables|Default|GetSprite) "/Game/Texture/Walk/dotpict_walk_Flipbook.dotpict_walk_Flipbook")
        (else
          (Sprite|SetFlipbook (Variables|Default|GetSprite) "/Game/Texture/Stay/dotpict_Stay_Flipbook.dotpict_Stay_Flipbook"))))))