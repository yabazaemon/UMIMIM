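; BP_Lock is a clickable rock actor with hit points that registers itself in BP_GameState's live count (LeavesNowCount).
; Clicks while CanBreak is set reduce RockHP, and Tick destroys the actor once RockKilled or RockDefeated is true.
; EndPlay on destruction lowers the live count, adding score (doubled in OnAlmostzone) and a kill, or a death if defeated.
; LeafFlipTurn mirrors the flipbook by horizontal movement but is not called here.
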(event OnClicked(ClickedCollision)
  (params (TouchedComponent :type Primitive%20Component%20Object%20Reference) (ButtonPressed :type Key%20Structure :default "None"))
  (if (Variables|Default|GetCanBreak)
    (Variables|Default|SetRockHP (- (Variables|Default|GetRockHP) 1))
    (if (<= (Variables|Default|GetRockHP) 0)
      (Variables|Default|SetRockKilled true))))

(event EventBeginPlay
  (Variables|Default|SetRockKilled false)
  (Variables|Default|SetRockDefeated false)
  (bind _asbp_game_state (Utilities|Casting|CastToBP_GameState (Game|GetGameState)))
  (Variables|/Game/BluePrint/BP_GameState.BP_GameState_C|SetLeavesNowCount _asbp_game_state (+ (Variables|/Game/BluePrint/BP_GameState.BP_GameState_C|GetLeavesNowCount _asbp_game_state) 1)))

(event Collision|EventActorBeginOverlap
  (params (OtherActor :type Actor%20Object%20Reference)))

(event EventTick
  (params (DeltaSeconds :type Float%20%28single-precision%29))
  (if (Variables|Default|GetRockKilled)
    (Actor|DestroyActor)
    (elif (Variables|Default|GetRockDefeated)
      (Actor|DestroyActor))))

(event EventEndPlay
  (params (EndPlayReason :type EEndPlayReason%20Enum :default "Destroyed"))
  (switch Utilities|FlowControl|Switch|SwitchonEEndPlayReason EndPlayReason
    (:Destroyed
      (if (Variables|Default|GetRockKilled)
        (bind _asbp_game_state (Utilities|Casting|CastToBP_GameState (Game|GetGameState)))
        (if (Variables|Default|GetOn%20almostzone)
          (bind _output_get (Variables|/Game/BluePrint/BP_GameState.BP_GameState_C|SetScore _asbp_game_state (+ (Variables|/Game/BluePrint/BP_GameState.BP_GameState_C|GetScore _asbp_game_state) (* (Variables|Default|GetNomal%20Rock%20Score) 2))))
          (Development|PrintString (Utilities|String|ToString(Integer) _output_get))
          (Variables|Default|SetRockKilled false)
          (bind _asbp_game_state_2 (Utilities|Casting|CastToBP_GameState (Game|GetGameState)))
          (bind _output_get_2 (Variables|/Game/BluePrint/BP_GameState.BP_GameState_C|SetLeavesNowCount _asbp_game_state_2 (- (Variables|/Game/BluePrint/BP_GameState.BP_GameState_C|GetLeavesNowCount _asbp_game_state_2) 1)))
          (Development|PrintString (Utilities|String|ToString(Integer) _output_get_2))
          (bind _output_get_3 (Variables|/Game/BluePrint/BP_GameState.BP_GameState_C|SetKillCount _asbp_game_state_2 (+ (Variables|/Game/BluePrint/BP_GameState.BP_GameState_C|GetKillCount _asbp_game_state_2) 1)))
          (Development|PrintString (Utilities|String|ToString(Integer) _output_get_3))
          (else
            (bind _output_get_4 (Variables|/Game/BluePrint/BP_GameState.BP_GameState_C|SetScore _asbp_game_state (+ (Variables|/Game/BluePrint/BP_GameState.BP_GameState_C|GetScore _asbp_game_state) (Variables|Default|GetNomal%20Rock%20Score))))
            (Development|PrintString (Utilities|String|ToString(Integer) _output_get_4))
            (Variables|Default|SetRockKilled false)
            (bind _asbp_game_state_3 (Utilities|Casting|CastToBP_GameState (Game|GetGameState)))
            (bind _output_get_5 (Variables|/Game/BluePrint/BP_GameState.BP_GameState_C|SetLeavesNowCount _asbp_game_state_3 (- (Variables|/Game/BluePrint/BP_GameState.BP_GameState_C|GetLeavesNowCount _asbp_game_state_3) 1)))
            (Development|PrintString (Utilities|String|ToString(Integer) _output_get_5))
            (bind _output_get_6 (Variables|/Game/BluePrint/BP_GameState.BP_GameState_C|SetKillCount _asbp_game_state_3 (+ (Variables|/Game/BluePrint/BP_GameState.BP_GameState_C|GetKillCount _asbp_game_state_3) 1)))
            (Development|PrintString (Utilities|String|ToString(Integer) _output_get_6))))
        (elif (Variables|Default|GetRockDefeated)
          (bind _asbp_game_state_4 (Utilities|Casting|CastToBP_GameState (Game|GetGameState)))
          (bind _output_get_7 (Variables|/Game/BluePrint/BP_GameState.BP_GameState_C|SetDeathCount _asbp_game_state_4 (+ (Variables|/Game/BluePrint/BP_GameState.BP_GameState_C|GetDeathCount _asbp_game_state_4) 1)))
          (Development|PrintString (Utilities|String|ToString(Integer) _output_get_7))
          (bind _asbp_game_state_5 (Utilities|Casting|CastToBP_GameState (Game|GetGameState)))
          (bind _output_get_8 (Variables|/Game/BluePrint/BP_GameState.BP_GameState_C|SetLeavesNowCount _asbp_game_state_5 (- (Variables|/Game/BluePrint/BP_GameState.BP_GameState_C|GetLeavesNowCount _asbp_game_state_5) 1)))
          (Development|PrintString (Utilities|String|ToString(Integer) _output_get_8))
          (else
            (bind _asbp_game_state_6 (Utilities|Casting|CastToBP_GameState (Game|GetGameState)))
            (bind _output_get_9 (Variables|/Game/BluePrint/BP_GameState.BP_GameState_C|SetLeavesNowCount _asbp_game_state_6 (- (Variables|/Game/BluePrint/BP_GameState.BP_GameState_C|GetLeavesNowCount _asbp_game_state_6) 1)))
            (Development|PrintString (Utilities|String|ToString(Integer) _output_get_9))))))))

(fn ConstructionScript)

(fn LeafFlipTurn
  (params (Delta%20Seconds :type Float%20%28double-precision%29))
  (bind _output_get (Variables|Default|SetCurrentLocation (Transformation|GetActorLocation)))
  (Math|Float|CompareFloat (.X (Math|Vector|BreakVector (- _output_get (Variables|Default|GetPreviousLocation)))) 0.0
    (:>
      (Transformation|SetRelativeScale3D (Variables|Default|GetFlipbook) "-1.000000,1.000000,1.000000")
      (Variables|Default|SetPreviousLocation (Variables|Default|GetCurrentLocation)))
    (:<
      (Transformation|SetRelativeScale3D (Variables|Default|GetFlipbook) "1.000000,1.000000,1.000000")
      (Variables|Default|SetPreviousLocation (Variables|Default|GetCurrentLocation)))))